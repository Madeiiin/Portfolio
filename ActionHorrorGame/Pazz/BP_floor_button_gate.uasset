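; BP_floor_button_gate is a gate whose static mesh slides open and closed in response to a floor button.
; On BeginPlay it finds a BP_floor_button through GetActorOfClass and binds its own Open and Close events to that button's dispatchers.
; Each event uses MoveComponentTo to shift the mesh along X in opposite directions, computing the relative-location target from the mesh's current world location.
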(event Custom|open
  (bind _staticmeshcomponent (Variables|Debug|GetStaticMeshComponent))
  (Components|MoveComponentTo _staticmeshcomponent (+ (Transformation|GetWorldLocation _staticmeshcomponent) "500.000000,0.000000,0.000000") "0, 0, 0" false false 0.2 false))

(event Custom|close
  (bind _staticmeshcomponent (Variables|Debug|GetStaticMeshComponent))
  (Components|MoveComponentTo _staticmeshcomponent (- (Transformation|GetWorldLocation _staticmeshcomponent) "500.000000,0.000000,0.000000") "0, 0, 0" false false 0.2 false))

(event EventBeginPlay
  (bind _returnvalue (Actor|GetActorOfClass "/Game/StoryAdvTemplate/Blueprints/Pazz/BP_floor_button.BP_floor_button_C"))
  (bind _output_get (Variables|Default|SetButton%20ref _returnvalue))
  (EventDispatchers|BindEventtoOpen _output_get (delegate Custom|open))
  (EventDispatchers|BindEventtoClose _output_get (delegate Custom|close)))

(fn ConstructionScript)